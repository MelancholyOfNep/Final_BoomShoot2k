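; BP_EnemyShooterFixed is an AI enemy character that reacts to seeing or being hurt by the player.
; Damage lowers Health, raises walk speeds through Alert, calls Detected, and destroys the actor at zero health.
; Perception updates for FirstPersonCharacter also call Detected, even on lost stimulus, setting blackboard SawPlayer true and playing a zombie sound once.
; A falling check that zeroes movement speed is unconnected and never runs.
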(event `self.ReceiveTick`
  (params (DeltaSeconds :type "Float (single-precision)")))

(event `self.ReceiveAnyDamage`
  (params (Damage :type "Float (single-precision)") (DamageType :type "DamageType Object Reference") (InstigatedBy :type "Controller Object Reference") (DamageCauser :type "Actor Object Reference"))
  (bind _health (`self.Health`))
  (set `self.Health` (- _health Damage))
  (`self.Alert`)
  (`self.Detected`)
  (if (<= _health 0.0)
    (`self.K2_DestroyActor`)))

(event `Alert`
  (bind _charactermovement (`self.CharacterMovement`))
  (set `CharacterMovementComponent.MaxWalkSpeed` 600.0 _charactermovement)
  (set `CharacterMovementComponent.MaxWalkSpeedCrouched` 300.0 _charactermovement))

(event `self.AIPerception.OnTargetPerceptionUpdated`
  (params (Actor :type "Actor Object Reference") (Stimulus :type "AIStimulus Structure"))
  (cast `/Game/FirstPersonBP/Blueprints/FirstPersonCharacter` Actor)
  (set `self.Detected Player` (`.bSuccessfullySensed` (break `AIStimulus` Stimulus)))
  (`self.Detected`))

(event `Detected`
  (`BlackboardComponent.SetValueAsBool` (`AIBlueprintHelperLibrary.GetBlackboard` null) "SawPlayer" true)
  (if (not (stale _output_get))
    (bind _output_get (set `self.check` true))
    (`GameplayStatics.PlaySoundAtLocation` "/Game/fastzombie1.fastzombie1" (`SceneComponent.K2_GetComponentLocation` (`self.CapsuleComponent`)) (struct) 0.7 1.0 0.0 null null null)))

(fn `UserConstructionScript`)