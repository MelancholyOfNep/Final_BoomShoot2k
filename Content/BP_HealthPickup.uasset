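; BP_HealthPickup is a collectible that restores health to the first-person player character on touch.
; A sphere overlap casts the other actor to FirstPersonCharacter and skips characters already at full health, leaving the pickup in place.
; Otherwise it adds a fixed amount capped at the maximum, calls Healed and the UI widget's Pickup, then destroys itself.
; Non-player overlaps only print a debug message.
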(event `self.Sphere Collision.OnComponentBeginOverlap`
  (params (OverlappedComponent :type "PrimitiveComponent Object Reference") (OtherActor :type "Actor Object Reference") (OtherComp :type "PrimitiveComponent Object Reference") (OtherBodyIndex :type Integer) (bFromSweep :type Boolean) (SweepResult :type "HitResult Structure (by ref)"))
  (bind _asfirst_person_character (cast `/Game/FirstPersonBP/Blueprints/FirstPersonCharacter` OtherActor)
    (:`then`
      (bind _output_get (set `self.FPCharacterRef` _asfirst_person_character))
      (bind _health (`/Game/FirstPersonBP/Blueprints/FirstPersonCharacter.Health` _output_get))
      (if (not (>= _health 100.0))
        (if (>= _health 80.0)
          (set `/Game/FirstPersonBP/Blueprints/FirstPersonCharacter.Health` 100.0 _output_get)
          (else
            (set `/Game/FirstPersonBP/Blueprints/FirstPersonCharacter.Health` (+ _health 20.0) _output_get)))
        (`/Game/FirstPersonBP/Blueprints/FirstPersonCharacter.Healed` _output_get)
        (`/Game/Widgets/PlayerUI.Pickup` (`/Game/FirstPersonBP/Blueprints/FirstPersonCharacter.PlayerUIWidget` _output_get))
        (`self.K2_DestroyActor`)))
    (:`CastFailed`
      (`KismetSystemLibrary.PrintString` "Not the player"))))

(fn `UserConstructionScript`)